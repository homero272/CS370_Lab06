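; Boo is a ghost actor that creeps toward the player while off screen and stops when it is rendered.
; Each tick it turns to face the player, uses WasRecentlyRendered as the visibility test, and moves with VInterpTo without sweep when unseen.
; A timeline plays when seen and reverses when unseen, driving the Translucency parameter on a dynamic material instance.
; BeginPlay creates that material and adds a HUD widget to the viewport.
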(event EventBeginPlay
  (bind _returnvalue (Rendering|Material|CreateDynamicMaterialInstance (Variables|Default|Getboo) 0 0 "None" :!class /Script/Engine.PrimitiveComponent))
  (Variables|Default|SetTranslucent%20Material%20Instance _returnvalue)
  (bind _returnvalue_2 (UserInterface|CreateWidget "/Game/Blueprints/HUD.HUD_C"))
  (UserInterface|Viewport|AddtoViewport _returnvalue_2 0))

(event Collision|EventActorBeginOverlap
  (params (OtherActor :type Actor%20Object%20Reference)))

(event EventTick
  (params (DeltaSeconds :type Float%20%28single-precision%29))
  (bind _returnvalue (Game|GetPlayerCharacter 0))
  (bind _boo (Variables|Default|Getboo))
  (bind _returnvalue_2 (Transformation|GetActorLocation _returnvalue))
  (Transformation|SetActorRelativeRotation (Math|Conversions|RotationFromXVector (Math|Vector|Lerp(Vector) (Math|Vector|GetForwardVector _boo) (- _returnvalue_2 (Transformation|GetWorldLocation _boo)) 1.0)))
  (if (Class|Actor|WasRecentlyRendered 0.2)
    (bind _newtrack_0 (Timeline|translucency_timeline Play)
      (:Update
        (Rendering|Material|SetScalarParameterValue (Variables|Default|GetTranslucent%20Material%20Instance) "Translucency" _newtrack_0 :!class /Script/Engine.MaterialInstanceDynamic)))
    (else
      (Transformation|SetActorLocation (Math|Interpolation|VInterpTo (Transformation|GetWorldLocation (Variables|Default|Getboo)) _returnvalue_2 DeltaSeconds 0.5) false false)
      (Timeline|translucency_timeline Reverse))))

(event EventInterfaceEvent)

(fn ConstructionScript)