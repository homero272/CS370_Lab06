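; BP_Character is a player character that looks with the mouse, interacts with objects and teleports to where it is looking.
; Each tick, a camera line trace stores either an actor implementing BP_InteractionInterface or a hit location that permits teleporting.
; The interact/teleport action messages that actor, or otherwise moves the character to the hit point with a vertical offset.
; A Move helper exists but is not called in these graphs.
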(event Custom|GazeCheck
  (bind _camera (Variables|Default|GetCamera))
  (bind _returnvalue (Transformation|GetWorldLocation _camera))
  ;[1 1 1] Gaze check
  (bind _outhit (Collision|LineTraceByChannel _returnvalue (+ _returnvalue (* (Math|Vector|GetForwardVector _camera) 2000)) "TraceTypeQuery1" false 0 "ForOneFrame"))
  (if (Utilities|DoesObjectImplementInterface (.HitActor (Collision|BreakHitResult _outhit)) "/Game/Blueprints/BP_InteractionInterface.BP_InteractionInterface_C")
    (Variables|Default|SetinteractingActor (.HitActor (Collision|BreakHitResult _outhit)))
    (Variables|Default|SetcanMove false)
    (else
      (Variables|Default|SetinteractingActor 0)
      (Variables|Default|SethitLocation (.Location (Collision|BreakHitResult _outhit)))
      (Variables|Default|SetcanMove true))))

(event EventTick
  (params (DeltaSeconds :type Float%20%28single-precision%29))
  (CallFunction|GazeCheck))

(event Input|ActionEvents|InputActioninteract/teleport
  (params (Key :type Key%20Structure :default "None"))
  (bind _interactingactor (Variables|Default|GetinteractingActor))
  (:Pressed
    (Utilities|IsValid _interactingactor
      (:Is%20Valid
        (Class|BPInteractionInterface|InterfaceEvent(Message) _interactingactor))
      (:Is%20Not%20Valid
        (CallFunction|Teleport)))))

(event Input|AxisEvents|InputAxismouseX
  (params (AxisValue :type Float%20%28single-precision%29))
  ;[1 1 1] Input
  (Pawn|Input|AddControllerYawInput AxisValue))

(event Input|AxisEvents|InputAxismouseY
  (params (AxisValue :type Float%20%28single-precision%29))
  ;[1 1 1] Input
  (Pawn|Input|AddControllerPitchInput AxisValue))

(event Input|AxisEvents|InputAxisMouseCursor
  (params (AxisValue :type Float%20%28single-precision%29))
  ;[1 1 1] Input
)

(fn ConstructionScript)

(fn Move
  (params (axisVal :type Float%20%28double-precision%29) (speed :type Float%20%28double-precision%29))
  (Pawn|Input|AddMovementInput (* speed (Transformation|GetActorForwardVector) (Variables|Default|GetSpeed)) axisVal false))

(fn Teleport
  (if (Variables|Default|GetcanMove)
    (Transformation|SetActorLocation (+ (Variables|Default|GethitLocation) "0,0,88.000000") false false)))